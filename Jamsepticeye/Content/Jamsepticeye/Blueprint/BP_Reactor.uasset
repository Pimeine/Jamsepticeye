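; Reactor actor that acts as a win objective: deactivating it with the matching glyph wins the game.
; On BeginPlay it finds BP_TimeManager and binds to its end-of-time and time-to-explode events; end of time starts a looping mesh animation, while the explode handler is empty.
; ValidGlyph compares the glyph name to one skill enum value, then Deactivated plays the death animation and calls GameWin on the manager after a delay.
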(event Custom|EOT
  (Components|Animation|PlayAnimation (Variables|Default|GetSkeletalMesh) 0 true))

(event Custom|TimeToExplode_Event_0)

(event Custom|Deactivated
  (Components|Animation|PlayAnimation (Variables|Default|GetSkeletalMesh) "/Game/Jamsepticeye/Environment/Models/Reacteur_Animated_02_Anim_Armature_Death.Reacteur_Animated_02_Anim_Armature_Death" false)
  (Utilities|FlowControl|Delay 5.0)
  (Default|GameWin (Variables|Default|GetTimeManager)))

(event EventBeginPlay
  (bind _returnvalue (Actor|GetActorOfClass "/Game/Jamsepticeye/Blueprint/TimeSystem/BP_TimeManager.BP_TimeManager_C"))
  (bind _output_get (Variables|Default|SetTimeManager _returnvalue))
  (EventDispatchers|BindEventtoEndOfTime _output_get (delegate Custom|EOT))
  (EventDispatchers|AssignTimetoExplode _output_get (delegate Custom|TimeToExplode_Event_0)))

(event EventValidGlyph
  (params (GlyphName :type String))
  (if (CallFunction|Equal(String,EnumSkill) GlyphName "NewEnumerator4")
    (CallFunction|Deactivated)))

(fn ConstructionScript)