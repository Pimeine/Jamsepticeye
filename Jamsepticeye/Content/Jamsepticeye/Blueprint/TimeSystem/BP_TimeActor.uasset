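; Base actor for the time system that returns to its saved checkpoint transform when time runs out.
; On BeginPlay it binds to BP_TimeManager's end-of-time and update events and caches the player pawn, also listening for BP_PlayerStart's spawn event.
; Updates store its transform by checkpoint index; end of time teleports it to the player's last checkpoint entry, a default meant for child overrides.
; The construction script toggles mesh physics via IsPhysicActor.
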(event Custom|EndOfTime
  ;[0 0 0] End Of Time
  (CallFunction|EOTReturn (Variables|/Game/HTML_Template/Blueprint/Player/BP_TP_PlayerPawn.BP_TP_PlayerPawn_C|GetLastCheckpointIndex (Variables|Default|GetPlayerPawn))))

(event Custom|UpdateTimeStamp
  (params (CheckpointIndex :type Integer))
  ;[0 0 0] Exemple, will probably be overided on Childs
  (Utilities|Map|Add (Variables|Default|GetSavedTransform) CheckpointIndex (Transformation|GetActorTransform)))

(event Custom|EOT_Return
  (params (CheckpointIndex :type Integer))
  ;[0 0 0] Exemple, will probably be overided on Childs
  (Transformation|SetActorTransform (.Value (Utilities|Map|Find (Variables|Default|GetSavedTransform) CheckpointIndex)) false true))

(event Custom|GetPlayer
  (bind _asbp_tp_player_pawn (Utilities|Casting|CastToBP_TP_PlayerPawn (Game|Player|GetPlayerPawn 0)))
  (Variables|Default|SetPlayerPawn _asbp_tp_player_pawn))

(event EventBeginPlay
  (bind _returnvalue (Actor|GetActorOfClass "/Game/Jamsepticeye/Blueprint/TimeSystem/BP_TimeManager.BP_TimeManager_C"))
  (bind _output_get (Variables|Default|SetTimeManager _returnvalue))
  (EventDispatchers|BindEventtoEndOfTime _output_get (EventDispatchers|CreateEvent :!event Custom|EndOfTime))
  (EventDispatchers|BindEventtoUpdateTimeActor _output_get (EventDispatchers|CreateEvent :!event Custom|UpdateTimeStamp))
  (bind _returnvalue_2 (Actor|GetActorOfClass "/Game/HTML_Template/Blueprint/Player/BP_PlayerStart.BP_PlayerStart_C"))
  (EventDispatchers|BindEventtoPlayerSpawned _returnvalue_2 (delegate Custom|GetPlayer))
  (Variables|Default|GetPlayerPawn
    (:then)
    (:else
      (bind _asbp_tp_player_pawn (Utilities|Casting|CastToBP_TP_PlayerPawn (Game|Player|GetPlayerPawn 0)))
      (Variables|Default|SetPlayerPawn _asbp_tp_player_pawn))))

(fn ConstructionScript
  (bind _staticmesh (Variables|Default|GetStaticMesh))
  (if (Variables|Default|GetbIsPhysicActor)
    (Physics|SetSimulatePhysics _staticmesh true)
    (else
      (Physics|SetSimulatePhysics _staticmesh false))))