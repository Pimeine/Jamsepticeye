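; Time manager that runs the game's countdown clock, binding to BP_PlayerStart's player-spawned event to start it.
; A looping one-second timer decrements CurrentTime, then at zero clears itself and fires EndOfTime after a short death-sequence delay.
; Reaching a checkpoint overrides both current and end time, so later restarts reuse that value.
; Game start and checkpoint updates broadcast UpdateTimeActor with the checkpoint index.
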(event Custom|UpdateTimeClock
  (bind _output_get (Variables|Default|SetCurrentTime (- (Variables|Default|GetCurrentTime) 1)))
  (if (<= _output_get 0)
    (Utilities|Time|ClearandInvalidateTimerbyHandle (Variables|Default|GetTimeClockTimer))
    (Utilities|FlowControl|Delay 0.2 :!pinned true) ; EOT Delay - Used for Death Sequence Delay
    (Default|CallEndOfTime)))

(event Custom|StartGameTime
  (Variables|Default|SetCurrentTime (Variables|Default|GetEndTime))
  (Default|CallUpdateTimeActor)
  (bind _returnvalue (Utilities|Time|SetTimerbyEvent (EventDispatchers|CreateEvent :!event Custom|UpdateTimeClock) 1.0 true))
  (Variables|Default|SetTimeClockTimer _returnvalue))

(event Custom|ForceUpdateClock
  (params (CurrentTime :type Integer) (CheckpointIndex :type Integer))
  (bind _output_get (Variables|Default|SetCurrentTime CurrentTime))
  (Variables|Default|SetEndTime _output_get)
  (CallFunction|RestartClock)
  (Default|CallUpdateTimeActor CheckpointIndex))

(event Custom|RestartClock
  (Variables|Default|SetCurrentTime (Variables|Default|GetEndTime))
  (bind _returnvalue (Utilities|Time|SetTimerbyEvent (EventDispatchers|CreateEvent :!event Custom|UpdateTimeClock) 1.0 true))
  (Variables|Default|SetTimeClockTimer _returnvalue))

(event EventBeginPlay
  ;[0 0 0] Tart rhe first Timer when the player pawn Spawn
  (bind _returnvalue (Actor|GetActorOfClass "/Game/HTML_Template/Blueprint/Player/BP_PlayerStart.BP_PlayerStart_C"))
  (EventDispatchers|BindEventtoPlayerSpawned _returnvalue (EventDispatchers|CreateEvent :!event Custom|StartGameTime)))

(fn ConstructionScript)