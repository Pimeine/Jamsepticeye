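; Time-system door actor that swings open when it receives a glyph matching a specific skill.
; A valid glyph plays a transient sound and instantly sets the Door component's relative yaw or axis rotation to the open pose.
; On each timestamp update it stores the door's world transform by checkpoint index, and on EOTReturn teleports the door back to that saved transform, extending the parent's handling of both events.
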(event Custom|OpenDoor
  ;[0 0 0] Door Opening
  (CallFunction|AMPlayTransientSound "Enum_TranscientAudio_MAX" "0, 0, 0" "0, 0, 0" :!pinned true) ; SOUND: Door Opening
  (Transformation|SetRelativeRotation (Variables|Default|GetDoor) "0,120.000000, 0" false false))

(event EventBeginPlay
  (|CallParentFunction))

(event EventEOTReturn
  (params (CheckpointIndex :type Integer))
  ;[0 0.2407 1] RETURN
  (|CallParentFunction CheckpointIndex)
  (Transformation|SetWorldTransform (Variables|Default|GetDoor) (.Value (Utilities|Map|Find (Variables|Default|GetDoorTransform) CheckpointIndex)) false true))

(event EventUpdateTimeStamp
  (params (CheckpointIndex :type Integer))
  ;[0 0.2407 1] UPDATE
  (|CallParentFunction CheckpointIndex)
  (Utilities|Map|Add (Variables|Default|GetDoorTransform) CheckpointIndex (Transformation|GetWorldTransform (Variables|Default|GetDoor))))

(event EventValidGlyph
  (params (GlyphName :type String))
  ;[0 0.2407 1] Check Glyph
  (if (CallFunction|Equal(String,EnumSkill) GlyphName "NewEnumerator0")
    (CallFunction|OpenDoor)))

(fn ConstructionScript)