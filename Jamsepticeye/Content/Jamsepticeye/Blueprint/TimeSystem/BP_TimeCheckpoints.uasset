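; BP_TimeCheckpoints is a checkpoint actor that records player progress and forces the game clock to a set time.
; When the player pawn first overlaps its collider, it passes its transform and index to the pawn, activates, and calls ForceUpdateClock on the pawn's time manager.
; Activation turns the cylinder green; the construction script can pre-activate it and computes a raised CheckpointTransform, though overlap passes the raw actor transform.
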(event OnComponentBeginOverlap(CheckpointCollider)
  (params (OverlappedComponent :type Primitive%20Component%20Object%20Reference) (OtherActor :type Actor%20Object%20Reference) (OtherComp :type Primitive%20Component%20Object%20Reference) (OtherBodyIndex :type Integer) (bFromSweep :type Boolean) (SweepResult :type Hit%20Result%20Structure%20%28by%20ref%29))
  (if (not (Variables|Default|GetbActivated))
    (bind _asbp_tp_player_pawn (Utilities|Casting|CastToBP_TP_PlayerPawn OtherActor))
    (Default|UpdateLastCheckpoint _asbp_tp_player_pawn (Transformation|GetActorTransform) (Variables|Default|GetCheckpointIndex))
    (CallFunction|ActivateCheckpoint true)
    (Default|ForceUpdateClock (Variables|/Game/HTML_Template/Blueprint/Player/BP_TP_PlayerPawn.BP_TP_PlayerPawn_C|GetTimeManagerActor _asbp_tp_player_pawn) (Variables|Default|GetForcedClockTime) (Variables|Default|GetCheckpointIndex))))

(event EventBeginPlay)

(fn ConstructionScript
  (CallFunction|ActivateCheckpoint (Variables|Default|GetForceActivation))
  (Variables|Default|SetCheckpointTransform (Math|Transform|MakeTransform (+ (Transformation|GetActorLocation) "0, 0,200.000000") (Transformation|GetActorRotation) "1,1,1")))

(fn ActivateCheckpoint
  (params (bIsActivated :type Boolean))
  (bind _output_get (Variables|Default|SetbActivated bIsActivated))
  (if _output_get
    ;[1 0 0] MUST: be changed
    (Rendering|Material|SetMaterial (Variables|Default|GetCylinder) 0 "/AnimationSharing/AnimSharingGreen.AnimSharingGreen")))