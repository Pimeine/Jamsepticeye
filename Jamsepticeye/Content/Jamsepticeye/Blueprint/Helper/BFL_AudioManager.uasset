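; Blueprint function library that centralizes game audio setup, playback and musical pitch helpers.
; Audio components and one-shot spatial or 2D sounds take their settings from enum-keyed rows in DT_AudioComponents and DT_TranscientAudio, with random-pitch variants for component and spatial sounds.
; A crossfade helper swaps two components.
; TuneToNote converts a degree in a chosen scale to a pitch multiplier by raising a semitone constant to the looked-up scale value.
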(fn AMInitializeAudioComp
  (params (AudioComponent :type Audio%20Component%20Object%20Reference) (AudioName :type Enum_AudioComponents%20Enum :default "Enum_AudioComponents_MAX"))
  (bind _returnvalue (Utilities|GetDataTableRow "/Game/Jamsepticeye/Blueprint/Audio/DT_AudioComponents.DT_AudioComponents" (Utilities|Name|EnumtoName AudioName))
    (:then
      (Audio|Components|Audio|SetSound AudioComponent (.Sound (Utilities|Struct|BreakStruct_AudioComponent _returnvalue)))
      (Variables|/Script/Engine.AudioComponent|SetbOverrideSubtitlePriority AudioComponent (.OverrideSubtitlePriority (Utilities|Struct|BreakStruct_AudioComponent _returnvalue)))
      (Variables|/Script/Engine.AudioComponent|SetbIsUISound AudioComponent (.IsUISound (Utilities|Struct|BreakStruct_AudioComponent _returnvalue)))
      (Variables|/Script/Engine.AudioComponent|SetbOverridePriority AudioComponent (.OverridePriority (Utilities|Struct|BreakStruct_AudioComponent _returnvalue)))
      (Variables|/Script/Engine.AudioComponent|SetbSuppressSubtitles AudioComponent (.SupressSubtitles (Utilities|Struct|BreakStruct_AudioComponent _returnvalue)))
      (Variables|/Script/Engine.AudioComponent|SetVolumeMultiplier AudioComponent (.VolumeMultiplier (Utilities|Struct|BreakStruct_AudioComponent _returnvalue)))
      (Variables|/Script/Engine.AudioComponent|SetPitchMultiplier AudioComponent (.PitchMultiplier (Utilities|Struct|BreakStruct_AudioComponent _returnvalue)))
      (Variables|/Script/Engine.AudioComponent|SetbAllowSpatialization AudioComponent (.AllowSpatialization (Utilities|Struct|BreakStruct_AudioComponent _returnvalue)))
      (Variables|/Script/Engine.AudioComponent|SetAttenuationSettings AudioComponent (.AttenuationSettings (Utilities|Struct|BreakStruct_AudioComponent _returnvalue))))))

(fn AMInitializeAudioCompRandomPitch
  (params (AudioComponent :type Audio%20Component%20Object%20Reference) (AudioName :type Enum_AudioComponents%20Enum :default "Enum_AudioComponents_MAX"))
  (bind _returnvalue (Utilities|GetDataTableRow "/Game/Jamsepticeye/Blueprint/Audio/DT_AudioComponents.DT_AudioComponents" (Utilities|Name|EnumtoName AudioName))
    (:then
      (Audio|Components|Audio|SetSound AudioComponent (.Sound (Utilities|Struct|BreakStruct_AudioComponent _returnvalue)))
      (Variables|/Script/Engine.AudioComponent|SetbOverrideSubtitlePriority AudioComponent (.OverrideSubtitlePriority (Utilities|Struct|BreakStruct_AudioComponent _returnvalue)))
      (Variables|/Script/Engine.AudioComponent|SetbIsUISound AudioComponent (.IsUISound (Utilities|Struct|BreakStruct_AudioComponent _returnvalue)))
      (Variables|/Script/Engine.AudioComponent|SetbOverridePriority AudioComponent (.OverridePriority (Utilities|Struct|BreakStruct_AudioComponent _returnvalue)))
      (Variables|/Script/Engine.AudioComponent|SetbSuppressSubtitles AudioComponent (.SupressSubtitles (Utilities|Struct|BreakStruct_AudioComponent _returnvalue)))
      (Variables|/Script/Engine.AudioComponent|SetVolumeMultiplier AudioComponent (.VolumeMultiplier (Utilities|Struct|BreakStruct_AudioComponent _returnvalue)))
      (Variables|/Script/Engine.AudioComponent|SetPitchMultiplier AudioComponent (Math|Random|RandomFloatinRange (.PitchMin (Utilities|Struct|BreakStruct_AudioComponent _returnvalue)) (.PitchMax (Utilities|Struct|BreakStruct_AudioComponent _returnvalue))))
      (Variables|/Script/Engine.AudioComponent|SetbAllowSpatialization AudioComponent (.AllowSpatialization (Utilities|Struct|BreakStruct_AudioComponent _returnvalue)))
      (Variables|/Script/Engine.AudioComponent|SetAttenuationSettings AudioComponent (.AttenuationSettings (Utilities|Struct|BreakStruct_AudioComponent _returnvalue))))))

(fn AMPlayTransientSound
  (params (Audio%20Name :type Enum_TranscientAudio%20Enum :default "Enum_TranscientAudio_MAX") (Location :type Vector) (Rotation :type Rotator))
  (bind _returnvalue (Utilities|GetDataTableRow "/Game/Jamsepticeye/Blueprint/Audio/DT_TranscientAudio.DT_TranscientAudio" (Utilities|Name|EnumtoName Audio%20Name))
    (:then
      (Audio|SpawnSoundatLocation (LocalVariables|Get__WorldContext) (.Sound (Utilities|Struct|BreakStruct_TranscientAudio _returnvalue)) Location Rotation (.VolumeMultiplier (Utilities|Struct|BreakStruct_TranscientAudio _returnvalue)) (.PitchMultiplier (Utilities|Struct|BreakStruct_TranscientAudio _returnvalue)) 0.0 (.AttenuationSettings (Utilities|Struct|BreakStruct_TranscientAudio _returnvalue)) (.ConcurrencySettings (Utilities|Struct|BreakStruct_TranscientAudio _returnvalue))))))

(fn AMPlayTransientSoundRandomPitch
  (params (Audio%20Name :type Enum_TranscientAudio%20Enum :default "Enum_TranscientAudio_MAX") (Location :type Vector) (Rotation :type Rotator))
  (bind _returnvalue (Utilities|GetDataTableRow "/Game/Jamsepticeye/Blueprint/Audio/DT_TranscientAudio.DT_TranscientAudio" (Utilities|Name|EnumtoName Audio%20Name))
    (:then
      (Audio|SpawnSoundatLocation (LocalVariables|Get__WorldContext) (.Sound (Utilities|Struct|BreakStruct_TranscientAudio _returnvalue)) Location Rotation (.VolumeMultiplier (Utilities|Struct|BreakStruct_TranscientAudio _returnvalue)) (Math|Random|RandomFloatinRange (.PitchMin (Utilities|Struct|BreakStruct_TranscientAudio _returnvalue)) (.PitchMax (Utilities|Struct|BreakStruct_TranscientAudio _returnvalue))) 0.0 (.AttenuationSettings (Utilities|Struct|BreakStruct_TranscientAudio _returnvalue)) (.ConcurrencySettings (Utilities|Struct|BreakStruct_TranscientAudio _returnvalue))))))

(fn AMPlaySound2D
  (params (Audio%20Name :type Enum_TranscientAudio%20Enum :default "Enum_TranscientAudio_MAX"))
  (bind _returnvalue (Utilities|GetDataTableRow "/Game/Jamsepticeye/Blueprint/Audio/DT_TranscientAudio.DT_TranscientAudio" (Utilities|Name|EnumtoName Audio%20Name))
    (:then
      (Audio|PlaySound2D (LocalVariables|Get__WorldContext) (.Sound (Utilities|Struct|BreakStruct_TranscientAudio _returnvalue)) (.VolumeMultiplier (Utilities|Struct|BreakStruct_TranscientAudio _returnvalue)) (.PitchMultiplier (Utilities|Struct|BreakStruct_TranscientAudio _returnvalue)) 0.0 (.ConcurrencySettings (Utilities|Struct|BreakStruct_TranscientAudio _returnvalue)) 0))))

(fn AMCrossFade
  (params (CurrentAudio :type Audio%20Component%20Object%20Reference) (NewAudio :type Audio%20Component%20Object%20Reference) (Fade%20Duration :type Float%20%28single-precision%29))
  (Audio|Components|Audio|FadeOut CurrentAudio Fade%20Duration 0.0 :!class /Script/Engine.AudioComponent)
  (Audio|Components|Audio|FadeIn NewAudio Fade%20Duration 1.0 0.0 :!class /Script/Engine.AudioComponent))

(fn AMTunetoNote
  (params (Degree :type Integer) (Mode :type EMusicMode%20Enum :default "NewEnumerator0"))
  (switch Utilities|FlowControl|Switch|SwitchonEMusicMode Mode
    (:NewEnumerator0
      (bind _returnvalue (CallFunction|AMGetPutch Degree (LocalVariables|GetMajor%20Scale%20ST)))
      (return _returnvalue))
    (:NewEnumerator1
      (bind _returnvalue_2 (CallFunction|AMGetPutch Degree (LocalVariables|GetMinor%20Scale%20ST)))
      (return _returnvalue_2))
    (:NewEnumerator2
      (bind _returnvalue_3 (CallFunction|AMGetPutch Degree (LocalVariables|GetMajor%20Penta%20Scale%20ST)))
      (return _returnvalue_3))
    (:NewEnumerator4
      (bind _returnvalue_4 (CallFunction|AMGetPutch Degree (LocalVariables|GetMinor%20Penta%20Scale%20ST)))
      (return _returnvalue_4))
    (:NewEnumerator3
      (bind _returnvalue_5 (CallFunction|AMGetPutch Degree (LocalVariables|GetToneScale)))
      (return _returnvalue_5))))

(fn AMScaleDegreetoPitch
  (params (Array :type Array%20of%20Integers) (Dimension%201 :type Integer))
  (return (Math|Float|Power (LocalVariables|GetPitchToSTConstant) (Math|Conversions|ToFloat(Integer) (Utilities|Array|Get(acopy) Array Dimension%201)))))

(fn AMGetSemiTonesfromDegree
  (params (A :type Integer) (TargetArray :type Array%20of%20Integers))
  (bind _returnvalue (Utilities|Array|Length TargetArray))
  (return (+ (* (/ A _returnvalue) 8) (Math|Integer|%(Integer) A _returnvalue))))

(fn AMGetPutch
  (params (A :type Integer) (TargetArray :type Array%20of%20Integers))
  (bind _returnvalue (CallFunction|AMGetSemiTonesfromDegree A TargetArray))
  (bind _returnvalue_2 (CallFunction|AMScaleDegreetoPitch 0 TargetArray _returnvalue))
  (return _returnvalue_2))