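; BP_GyphPage is an interactable glyph page whose image material and interaction radius are set in the construction script.
; A left click within range blends the view to the page and puts the player pawn in pad/book state; right click exits.
; Sphere overlaps toggle a control billboard and the pawn's camera focus.
; Glyph audio is configured from a data table, and input enabling is delayed to avoid accidental activation.
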(event OnComponentBeginOverlap(Sphere)
  (params (OverlappedComponent :type Primitive%20Component%20Object%20Reference) (OtherActor :type Actor%20Object%20Reference) (OtherComp :type Primitive%20Component%20Object%20Reference) (OtherBodyIndex :type Integer) (bFromSweep :type Boolean) (SweepResult :type Hit%20Result%20Structure%20%28by%20ref%29))
  (bind _asbp_tp_player_pawn (Utilities|Casting|CastToBP_TP_PlayerPawn OtherActor))
  (Default|FocusCamera _asbp_tp_player_pawn true)
  (Development|SetHiddeninGame (Variables|Default|GetControlBillboard) false false))

(event OnComponentEndOverlap(Sphere)
  (params (OverlappedComponent :type Primitive%20Component%20Object%20Reference) (OtherActor :type Actor%20Object%20Reference) (OtherComp :type Primitive%20Component%20Object%20Reference) (OtherBodyIndex :type Integer))
  (bind _asbp_tp_player_pawn (Utilities|Casting|CastToBP_TP_PlayerPawn OtherActor))
  (Default|FocusCamera _asbp_tp_player_pawn false)
  (Development|SetHiddeninGame (Variables|Default|GetControlBillboard) true false))

(event Custom|OnClickedPad
  (params (TouchedActor :type Actor%20Object%20Reference) (ButtonPressed :type Key%20Structure :default "None"))
  (if (== ButtonPressed "LeftMouseButton")
    (if (<= (Math|Vector|Distance(Vector) (Transformation|GetActorLocation (Game|Player|GetPlayerPawn 0)) (Transformation|GetActorLocation)) 2.5e+02)
      (bind _asbp_tp_player_pawn (Utilities|Casting|CastToBP_TP_PlayerPawn (Game|Player|GetPlayerPawn 0)))
      (bind _output_get (Variables|Default|SetPlayerPawn _asbp_tp_player_pawn))
      (Variables|/Game/HTML_Template/Blueprint/Player/BP_TP_PlayerPawn.BP_TP_PlayerPawn_C|SetPageRef _output_get self)
      (CallFunction|FocusonPad true))
    (elif (== ButtonPressed "RightMouseButton")
      (if (Variables|Default|GetbInPad)
        (Variables|/Game/HTML_Template/Blueprint/Player/BP_TP_PlayerPawn.BP_TP_PlayerPawn_C|SetPageRef (Variables|Default|GetPlayerPawn) 0)
        (CallFunction|FocusonPad false)))))

(event Custom|FocusOnPad
  (params (bIsFocus :type Boolean))
  (bind _returnvalue (Game|GetPlayerController 0))
  (if bIsFocus
    (Development|SetHiddeninGame (Variables|Default|GetControlBillboard) true false)
    (Game|Player|SetViewTargetwithBlend _returnvalue self 0.0 "VTBlend_Linear" 0.0 false)
    (bind _output_get (Variables|Default|SetbInPad true))
    (Default|ToggleinPadState (Variables|Default|GetPlayerPawn) _output_get true)
    (Utilities|FlowControl|Delay 0.3) ; Needed to not activate the sequence when entering
    (Input|EnableInput (Game|GetPlayerController 0))
    (else
      (Game|Player|SetViewTargetwithBlend _returnvalue (Game|Player|GetPlayerPawn 0) 0.0 "VTBlend_Linear" 0.0 false)
      (Variables|Default|SetbInPad false)
      (Default|ToggleinPadState (Variables|Default|GetPlayerPawn) false true)
      (Input|DisableInput (Game|GetPlayerController 0))
      (Utilities|Time|ClearandInvalidateTimerbyHandle (Variables|Default|GetCursorTracer))
      (if (Collision|IsOverlappingActor (Variables|Default|GetSphere) (Game|Player|GetPlayerPawn 0) :!class /Script/Engine.PrimitiveComponent)
        (Development|SetHiddeninGame (Variables|Default|GetControlBillboard) false false)
        (else
          (Development|SetHiddeninGame (Variables|Default|GetControlBillboard) true false))))))

(event EventBeginPlay
  (EventDispatchers|BindEventtoOnClicked (EventDispatchers|CreateEvent :!event Custom|OnClickedPad))
  (bind _returnvalue (Actor|GetActorOfClass "/Game/Jamsepticeye/Blueprint/TimeSystem/BP_TimeManager.BP_TimeManager_C"))
  (Variables|Default|SetTimeManager _returnvalue)
  (CallFunction|InitializeAudioComponent))

(fn ConstructionScript
  (Components|Sphere|SetSphereRadius (Variables|Default|GetSphere) (Variables|Default|GetInteractionRadius) false)
  (Rendering|Material|SetMaterial (Variables|Default|GetPlane) 0 (Utilities|Select :Index (Variables|Default|GetImageIndex) :Option%200 "/Game/Jamsepticeye/Blueprint/Glyph/Texture/MI_Arrow.MI_Arrow" :Option%201 "/Game/Jamsepticeye/Blueprint/Glyph/Texture/MI_Circle.MI_Circle" :Option%202 "/Game/Jamsepticeye/Blueprint/Glyph/Texture/MI_Door.MI_Door" :Option%203 "/Game/Jamsepticeye/Blueprint/Glyph/Texture/MI_Sword.MI_Sword")))

(fn InitializeAudioComponent
  (bind _glyphsound (Variables|Default|GetGlyphSound))
  (bind _returnvalue (Utilities|GetDataTableRow "/Game/Jamsepticeye/Blueprint/Audio/DT_TranscientAudio.DT_TranscientAudio" "GlyphesSFX")
    (:then
      (Audio|Components|Audio|SetSound _glyphsound (.Sound (Utilities|Struct|BreakStruct_TranscientAudio _returnvalue)))
      (Variables|/Script/Engine.AudioComponent|SetPitchMultiplier _glyphsound (Math|Random|RandomFloatinRange (.PitchMin (Utilities|Struct|BreakStruct_TranscientAudio _returnvalue)) (.PitchMax (Utilities|Struct|BreakStruct_TranscientAudio _returnvalue))))
      (Variables|/Script/Engine.AudioComponent|SetAttenuationSettings _glyphsound (.AttenuationSettings (Utilities|Struct|BreakStruct_TranscientAudio _returnvalue)))
      (Variables|/Script/Engine.AudioComponent|SetVolumeMultiplier _glyphsound (.VolumeMultiplier (Utilities|Struct|BreakStruct_TranscientAudio _returnvalue))))))