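; BP_GlyphPad is a clickable glyph pad actor that the player can zoom the view onto.
; BeginPlay binds an OnClicked handler, where a left click within 250 units of the player pawn focuses the pad and a right click releases it.
; FocusOnPad switches the player controller's view target between the pad and the pawn, tracking the state in InPad.
; The click handler also prints the pressed button's name.
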(event Custom|OnClickedPad
  (params (TouchedActor :type Actor%20Object%20Reference) (ButtonPressed :type Key%20Structure :default "None"))
  (Development|PrintString (Utilities|String|ToString(Text) (Class|KismetInputLibrary|KeyGetDisplayName ButtonPressed)))
  (if (== ButtonPressed "LeftMouseButton")
    (if (<= (Math|Vector|Distance(Vector) (Transformation|GetActorLocation (Game|Player|GetPlayerPawn 0)) (Transformation|GetActorLocation)) 2.5e+02)
      (CallFunction|FocusonPad true))
    (elif (== ButtonPressed "RightMouseButton")
      (CallFunction|FocusonPad false))))

(event Custom|FocusOnPad
  (params (bIsFocus :type Boolean))
  (bind _returnvalue (Game|GetPlayerController 0))
  (if bIsFocus
    (Game|Player|SetViewTargetwithBlend _returnvalue self 0.0 "VTBlend_Linear" 0.0 false)
    (Variables|Default|SetbInPad true)
    (else
      (Game|Player|SetViewTargetwithBlend _returnvalue (Game|Player|GetPlayerPawn 0) 0.0 "VTBlend_Linear" 0.0 false)
      (Variables|Default|SetbInPad false))))

(event EventBeginPlay
  (EventDispatchers|BindEventtoOnClicked (EventDispatchers|CreateEvent :!event Custom|OnClickedPad)))

(fn ConstructionScript)