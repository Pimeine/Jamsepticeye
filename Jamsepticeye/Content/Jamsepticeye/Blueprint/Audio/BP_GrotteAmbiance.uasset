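; Cave (grotte) ambience actor that starts playing its audio component when play begins.
; The construction script looks up the AMB_GrotteAmbiance row in DT_AudioComponents and assigns its sound to the component.
; Logic for random pitch, volume, attenuation and spatialization exists but is disconnected, so only the sound itself comes from the table.
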(event EventBeginPlay
  (Audio|Components|Audio|Play (Variables|Default|GetAudio) 0.0))

(event Collision|EventActorBeginOverlap
  (params (OtherActor :type Actor%20Object%20Reference)))

(event EventTick
  (params (DeltaSeconds :type Float%20%28single-precision%29)))

(fn ConstructionScript
  (bind _returnvalue (Utilities|GetDataTableRow "/Game/Jamsepticeye/Blueprint/Audio/DT_AudioComponents.DT_AudioComponents" "AMB_GrotteAmbiance")
    (:then
      (Audio|Components|Audio|SetSound (Variables|Default|GetAudio) (.Sound (Utilities|Struct|BreakStruct_AudioComponent _returnvalue))))))