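; Ambient sound actor for a mushroom that starts its Audio component when play begins.
; The construction script configures that component from the SFX_MushroomV2 row of DT_AudioComponents: sound, random pitch within the row's range, volume, UI flag and attenuation.
; The OverrideAttenuationManually flag sets the component's attenuation override; spatialization comes from the table only when that flag is off.
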(event EventBeginPlay
  (Audio|Components|Audio|Play (Variables|Default|GetAudio) 0.0))

(event Collision|EventActorBeginOverlap
  (params (OtherActor :type Actor%20Object%20Reference)))

(event EventTick
  (params (DeltaSeconds :type Float%20%28single-precision%29)))

(fn ConstructionScript
  (bind _audio (Variables|Default|GetAudio))
  (bind _overrideattenuationmanually (Variables|Default|GetOverrideAttenuationManually))
  (bind _audio_2 (Variables|Default|GetAudio))
  (bind _returnvalue (Utilities|GetDataTableRow "/Game/Jamsepticeye/Blueprint/Audio/DT_AudioComponents.DT_AudioComponents" "SFX_MushroomV2")
    (:then
      (Audio|Components|Audio|SetSound _audio_2 (.Sound (Utilities|Struct|BreakStruct_AudioComponent _returnvalue)))
      (Variables|/Script/Engine.AudioComponent|SetPitchMultiplier _audio_2 (Math|Random|RandomFloatinRange (.PitchMin (Utilities|Struct|BreakStruct_AudioComponent _returnvalue)) (.PitchMax (Utilities|Struct|BreakStruct_AudioComponent _returnvalue))))
      (Variables|/Script/Engine.AudioComponent|SetbIsUISound _audio_2 (.IsUISound (Utilities|Struct|BreakStruct_AudioComponent _returnvalue)))
      (Variables|/Script/Engine.AudioComponent|SetVolumeMultiplier _audio_2 (.VolumeMultiplier (Utilities|Struct|BreakStruct_AudioComponent _returnvalue)))
      (Variables|/Script/Engine.AudioComponent|SetAttenuationSettings _audio_2 (.AttenuationSettings (Utilities|Struct|BreakStruct_AudioComponent _returnvalue)))
      (if _overrideattenuationmanually
        (Variables|/Script/Engine.AudioComponent|SetbOverrideAttenuation _audio _overrideattenuationmanually)
        (else
          (Variables|/Script/Engine.AudioComponent|SetbOverrideAttenuation _audio _overrideattenuationmanually)
          (Variables|/Script/Engine.AudioComponent|SetbAllowSpatialization _audio_2 (.AllowSpatialization (Utilities|Struct|BreakStruct_AudioComponent _returnvalue))))))))