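; BP_DeathArea is a box trigger that starts the player's death sequence on overlap.
; At BeginPlay it finds and caches the level's BP_TimeManager.
; When a BP_TP_PlayerPawn enters, it overwrites the manager's CurrentTime with TimeBeforeDeath and plays the death montage.
; It also disables the pawn's movement and sets its DeathSequence flag.
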(event OnComponentBeginOverlap(Box)
  (params (OverlappedComponent :type Primitive%20Component%20Object%20Reference) (OtherActor :type Actor%20Object%20Reference) (OtherComp :type Primitive%20Component%20Object%20Reference) (OtherBodyIndex :type Integer) (bFromSweep :type Boolean) (SweepResult :type Hit%20Result%20Structure%20%28by%20ref%29))
  (bind _asbp_tp_player_pawn (Utilities|Casting|CastToBP_TP_PlayerPawn OtherActor))
  (Variables|/Game/Jamsepticeye/Blueprint/TimeSystem/BP_TimeManager.BP_TimeManager_C|SetCurrentTime (Variables|Default|GetTimeManager) (Variables|Default|GetTimeBeforeDeath))
  (Animation|PlayAnimMontage _asbp_tp_player_pawn "/Game/Jamsepticeye/Characters/Player/Anims/AM_Death.AM_Death" 1.0 "None")
  (Pawn|Components|CharacterMovement|SetMovementMode (Variables|/Script/Engine.Character|GetCharacterMovement _asbp_tp_player_pawn) "MOVE_None" 0)
  (Variables|/Game/HTML_Template/Blueprint/Player/BP_TP_PlayerPawn.BP_TP_PlayerPawn_C|SetbDeathSequence _asbp_tp_player_pawn true))

(event EventBeginPlay
  (bind _returnvalue (Actor|GetActorOfClass "/Game/Jamsepticeye/Blueprint/TimeSystem/BP_TimeManager.BP_TimeManager_C"))
  (Variables|Default|SetTimeManager _returnvalue))

(fn ConstructionScript)