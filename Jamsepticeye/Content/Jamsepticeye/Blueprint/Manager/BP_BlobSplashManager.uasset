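; Manager actor that spawns and removes blob splashes as instances of a single InstancedStaticMesh.
; On BeginPlay it finds BP_TimeManager and binds to its end-of-time and update-time-actor events.
; End of time removes instances listed in ToDestroy from highest index down, keeping remaining indices valid, while the update event clears that list.
; Nothing in this Blueprint fills ToDestroy.
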(event Custom|EOT_Update
  (params (Index :type Integer))
  (Utilities|Array|Clear (Variables|Default|GetToDestroy)))

(event Custom|EOT
  (CallFunction|SortList))

(event EventBeginPlay
  (bind _returnvalue (Actor|GetActorOfClass "/Game/Jamsepticeye/Blueprint/TimeSystem/BP_TimeManager.BP_TimeManager_C"))
  (bind _output_get (Variables|Default|SetTimeManager _returnvalue))
  (EventDispatchers|BindEventtoEndOfTime _output_get (EventDispatchers|CreateEvent :!event Custom|EOT))
  (EventDispatchers|BindEventtoUpdateTimeActor _output_get (EventDispatchers|CreateEvent :!event Custom|EOT_Update)))

(fn ConstructionScript)

(fn SpawnSplash
  (params (InstanceTransform :type Transform%20%28by%20ref%29))
  (bind _returnvalue (Components|InstancedStaticMesh|AddInstance (Variables|Default|GetInstancedStaticMesh) InstanceTransform))
  (return _returnvalue))

(fn ClearSplash
  (params (InstanceIndex :type Integer))
  (Class|InstancedStaticMeshComponent|RemoveInstance (Variables|Default|GetInstancedStaticMesh) InstanceIndex))

(fn SortList
  (bind _todestroy (Variables|Default|GetToDestroy))
  (bind (_indexofmaxvalue _maxvalue) (Math|Integer|MaxOfIntArray _todestroy))
  (Utilities|Array|ReverseforEachLoop (Variables|Default|GetToDestroy)
    (:LoopBody
      (CallFunction|ClearSplash _maxvalue)
      (Utilities|Array|RemoveIndex (Variables|Default|GetToDestroy) _indexofmaxvalue))))