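; Blueprint function library of shared helpers for the HTML game template, mostly routed through GI_HtmlGame and its GameData.
; It applies the project font to text, spawns the loading screen with optional audio fade, and prints prefixed debug messages.
; It also writes video settings to their save object, restores selected saves and hooks world setup into shader compilation.
; Game-data and privacy save functions only fetch objects, copying nothing.
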(fn HPrint
  (params (Message :type String) (TextColor :type Linear%20Color%20Structure :default "(R=0.000000,G=0.123422,B=1.000000,A=1.000000)") (Duration :type Float%20%28single-precision%29))
  (bind ___worldcontext (LocalVariables|Get__WorldContext))
  ;[0 0 0] Enhanced Print
  (Development|PrintString ___worldcontext (Utilities|String|Append (Utilities|GetObjectName ___worldcontext) " >> " Message) true true TextColor Duration))

(fn GetMyGameInstance
  (bind _asgi_html_game (Utilities|Casting|CastToGI_HtmlGame (Game|GetGameInstance)))
  (return _asgi_html_game))

(fn GetMyGameData
  (bind _asgi_html_game (Utilities|Casting|CastToGI_HtmlGame (Game|GetGameInstance)))
  (return (Variables|/Game/HTML_Template/Blueprint/Core/GI_HtmlGame.GI_HtmlGame_C|GetGameData _asgi_html_game)))

(fn SetTextStyle
  (params (TextTarget :type Text%20Block%20Object%20Reference))
  (bind _gamedata (CallFunction|GetMyGameData))
  (bind _font (Variables|/Script/UMG.TextBlock|GetFont TextTarget))
  (bind _font_2 (Variables|/Script/UMG.TextBlock|GetFont TextTarget))
  (Utilities|IsValid TextTarget
    (:Is%20Valid
      (Utilities|IsValid _gamedata
        (:Is%20Valid
          (Class|TextBlock|SetFont TextTarget (Utilities|Struct|MakeSlateFontInfo (Variables|/Game/HTML_Template/Blueprint/Core/DataAsset/PDA_Game.PDA_Game_C|GetTextFontFamily _gamedata) (.fontmaterial _font_2) (.outlinesettings _font_2) (.typefacefontname _font_2) (.size _font_2))))
        (:Is%20Not%20Valid
          (Class|TextBlock|SetFont TextTarget (Utilities|Struct|MakeSlateFontInfo (Variables|/Game/HTML_Template/Blueprint/Core/DataAsset/PDA_Game.PDA_Game_C|GetTextFontFamily (LocalVariables|GetDefaultGameData)) (.fontmaterial _font) (.outlinesettings _font) (.typefacefontname _font) (.size _font)) :!pinned true) ; Should Be Editor Only
        )))))

(fn HandleLoadingScreen
  (params (Loading%20Screen%20Mode :type Enum_LoadingScreenMode%20Enum :default "NewEnumerator0"))
  (LocalVariables|SetGameInstance (CallFunction|GetMyGameInstance))
  (if (Utilities|Enum|Equal(Enum) Loading%20Screen%20Mode "NewEnumerator0")
    (Variables|/Game/HTML_Template/Blueprint/Core/GI_HtmlGame.GI_HtmlGame_C|SetbIsLoadingScreen (LocalVariables|GetGameInstance) true)
    (Default|SetAudioSettings (LocalVariables|GetGameInstance) true "NewEnumerator0" 1.0))
  (bind _returnvalue (UserInterface|CreateWidget "/Game/HTML_Template/Blueprint/Widget/Manager/LoadingScreen/WBP_LoadingScreen.WBP_LoadingScreen_C" 0 (and (Utilities|Enum|Equal(Enum) Loading%20Screen%20Mode "NewEnumerator1") (not (Variables|/Game/HTML_Template/Blueprint/Core/GI_HtmlGame.GI_HtmlGame_C|GetbIsLoadingScreen (LocalVariables|GetGameInstance)))) Loading%20Screen%20Mode (Variables|/Game/HTML_Template/Blueprint/Core/DataAsset/PDA_Game.PDA_Game_C|GetLoadingScreenDuration (Variables|/Game/HTML_Template/Blueprint/Core/GI_HtmlGame.GI_HtmlGame_C|GetGameData (LocalVariables|GetGameInstance)))))
  (UserInterface|Viewport|AddtoViewport _returnvalue 9)
  (return _returnvalue))

(fn ConfigureVideoSettings
  (params (Framerate%20Target :type Enum_Video_FramerateTarget%20Enum :default "NewEnumerator0") (Anti%20Aliasing :type Enum_Video_AntiAliasing%20Enum :default "NewEnumerator0") (Shadow%20Quality :type Enum_Video_Shadow%20Enum :default "NewEnumerator0") (Texture%20Quality :type Enum_Video_TextureQuality%20Enum :default "NewEnumerator1") (Material%20Quality :type Enum_Video_MaterialQuality%20Enum :default "NewEnumerator1") (Bloom :type Enum_Video_Bloom%20Enum :default "NewEnumerator0") (ScreenPercent :type Enum_Video_ScreenPercent%20Enum :default "NewEnumerator4"))
  (LocalVariables|SetSavedVideoSettings (Default|GetVideoSavedSettings (CallFunction|GetMyGameInstance)))
  (Variables|/Game/HTML_Template/Save/Save_Video.Save_Video_C|SetFramerate (LocalVariables|GetSavedVideoSettings) Framerate%20Target)
  (Variables|/Game/HTML_Template/Save/Save_Video.Save_Video_C|SetAntiAliasing (LocalVariables|GetSavedVideoSettings) Anti%20Aliasing)
  (Variables|/Game/HTML_Template/Save/Save_Video.Save_Video_C|SetShadow (LocalVariables|GetSavedVideoSettings) Shadow%20Quality)
  (Variables|/Game/HTML_Template/Save/Save_Video.Save_Video_C|SetTextureQuality (LocalVariables|GetSavedVideoSettings) Texture%20Quality)
  (Variables|/Game/HTML_Template/Save/Save_Video.Save_Video_C|SetMaterialQuality (LocalVariables|GetSavedVideoSettings) Material%20Quality)
  (Variables|/Game/HTML_Template/Save/Save_Video.Save_Video_C|SetBloom (LocalVariables|GetSavedVideoSettings) Bloom)
  (Variables|/Game/HTML_Template/Save/Save_Video.Save_Video_C|SetScreenPercent (LocalVariables|GetSavedVideoSettings) ScreenPercent))

(fn LoadSaves
  (params (bLoadGameData :type Boolean) (bLoadVideo :type Boolean) (bLoadAudio :type Boolean) (bLoadShader :type Boolean) (bLoadPrivacy :type Boolean))
  (LocalVariables|SetGameInstance (CallFunction|GetMyGameInstance))
  (Utilities|FlowControl|Sequence
    (:then_0
      (if bLoadGameData
        (Save|LoadSaveGameData)))
    (:then_1
      (if bLoadVideo
        (Default|SetVideoSettings (LocalVariables|GetGameInstance))))
    (:then_2
      (if bLoadAudio
        (Default|SetAudioSettings (LocalVariables|GetGameInstance) false "NewEnumerator0" 0.0)))
    (:then_3
      (if bLoadShader
        (Save|LoadSaveShader)))
    (:then_4
      (if bLoadPrivacy
        (Save|LoadSavePrivacy)))))

(fn LoadSaveGameData
  (bind _asgi_html_game (CallFunction|GetMyGameInstance))
  (LocalVariables|SetSaveGameData (Default|GetGameDataSavedSettings _asgi_html_game))
  (LocalVariables|SetGameInstance _asgi_html_game))

(fn SetSaveGameData
  (bind _asgi_html_game (CallFunction|GetMyGameInstance))
  (LocalVariables|SetSaveGameData (Default|GetGameDataSavedSettings _asgi_html_game))
  (LocalVariables|SetGameInstance _asgi_html_game))

(fn LoadSavePrivacy
  (bind _asgi_html_game (CallFunction|GetMyGameInstance))
  (LocalVariables|SetSavePrivacy (Default|GetPrivacySavedSettings _asgi_html_game))
  (LocalVariables|SetGameInstance _asgi_html_game))

(fn SetSavePrivacy
  (bind _asgi_html_game (CallFunction|GetMyGameInstance))
  (LocalVariables|SetSavePrivacy (Default|GetPrivacySavedSettings _asgi_html_game))
  (LocalVariables|SetGameInstance _asgi_html_game))

(fn LoadSaveShader
  (bind _asgi_html_game (CallFunction|GetMyGameInstance))
  (LocalVariables|SetSaveShader (Default|GetShaderSavedSettings _asgi_html_game))
  (LocalVariables|SetGameInstance _asgi_html_game)
  (Variables|/Game/HTML_Template/Blueprint/Core/GI_HtmlGame.GI_HtmlGame_C|SetbFirstShaderCompiled (LocalVariables|GetGameInstance) (Variables|/Game/HTML_Template/Save/Save_Shader.Save_Shader_C|GetbFirstShaderCompiled (LocalVariables|GetSaveShader)))
  (Variables|/Game/HTML_Template/Blueprint/Core/GI_HtmlGame.GI_HtmlGame_C|SetCompiledLevelShader (LocalVariables|GetGameInstance) (Variables|/Game/HTML_Template/Save/Save_Shader.Save_Shader_C|GetCompiledLevelShader (LocalVariables|GetSaveShader))))

(fn SetCompilingShaderLevels
  (params (CompilingShaderLevels :type Array%20of%20World%20Soft%20Object%20References))
  (Variables|/Game/HTML_Template/Blueprint/Core/GI_HtmlGame.GI_HtmlGame_C|SetCompilingShaderLevels (CallFunction|GetMyGameInstance) CompilingShaderLevels))

(fn SetupWorld
  (params (ShaderText :type Text))
  (bind _asgi_html_game (CallFunction|GetMyGameInstance))
  (Utilities|Platform|CollectGarbage)
  (LocalVariables|SetGameInstance _asgi_html_game)
  (if (Variables|/Game/HTML_Template/Blueprint/Core/GI_HtmlGame.GI_HtmlGame_C|GetbIsCompilingShader _asgi_html_game)
    (Default|EConfigureLevelShaderCompilation (Variables|/Game/HTML_Template/Blueprint/Core/GI_HtmlGame.GI_HtmlGame_C|GetShaderLoadingscreenWidget (LocalVariables|GetGameInstance)) ShaderText)
    (Default|ERedrawCompilerWidget (LocalVariables|GetGameInstance))))

(fn Equal(String,EnumSkill)
  (params (SkillName :type String) (EnumSkill :type Enum_SkillNames%20Enum :default "NewEnumerator0"))
  (return (Utilities|Enum|Equal(Enum) SkillName (Utilities|String|EnumtoString EnumSkill))))