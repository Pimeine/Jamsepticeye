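; Game instance for the HTML game template, handling level loading, shader precompilation, music and saved settings across levels.
; Level changes run through loading-screen callbacks, crossfading into game music on game start.
; Shader precompilation opens levels under a compiler widget and saves which are done.
; Per-category save slots feed audio settings applied via sound mix overrides with optional fades, and video settings applied via console commands.
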(event Custom|E_OpenGameLevel
  (params (Level :type World%20Soft%20Object%20Reference))
  ;[0 0 0] Open Compiled Level with Loading Screen
  (bind _loading_screen_widget (CallFunction|HandleLoadingScreen "NewEnumerator0"))
  (EventDispatchers|BindEventtoOnLoadingComplete _loading_screen_widget (delegate Custom|OpeningGameLevel))
  (Variables|Default|SetLoadingScreenWidget _loading_screen_widget))

(event Custom|OpeningGameLevel
  ;[0 0 0] Open Compiled Level with Loading Screen
  (Class|Html5Library|OpenLevel(byObjectReference) (stale Custom|E_OpenGameLevel Level))
  (bind _returnvalue (Audio|SpawnSound2D (Variables|Audio|Music|GetGameMusic) 1.0 1.0 0.0 0 true false))
  (Variables|Default|SetSound_GameMusic _returnvalue)
  (CallFunction|AMCrossFade (Variables|Default|GetSound_MainMenuMusic) _returnvalue 2.0))

(event EventInit
  (CallFunction|InitializeGameData))

(event Custom|E_PerformShaderCompilation
  (params (TargetLevel :type World%20Soft%20Object%20Reference) (bIsLauncher :type Boolean))
  (Variables|Settings|SetLevelAfterCompilation TargetLevel)
  (bind _returnvalue (UserInterface|CreateWidget "/Game/HTML_Template/Blueprint/Widget/Manager/LoadingScreen/WBP_LoadingScreen_Shader.WBP_LoadingScreen_Shader_C"))
  (bind _output_get (Variables|Widget|SetShaderLoadingscreenWidget _returnvalue))
  (UserInterface|Viewport|AddtoViewport _output_get 10)
  (EventDispatchers|BindEventtoOnCompilationComplete _returnvalue (delegate Custom|ShaderCompilationFinished))
  (CallFunction|EOpenNextShaderLevel))

(event Custom|E_OpenNextShaderLevel
  ;[0 0 0] Open Next Shader To Compile
  (Class|Html5Library|OpenLevel(byObjectReference) (Utilities|Array|Get(acopy) (Variables|Settings|GetCompilingShaderLevels) (Variables|Settings|GetCurrentLevelToCompile))))

(event Custom|ShaderCompilationFinished
  (bind _save_shader (Variables|Save|GetSave_Shader))
  (Variables|Default|SetbIsCompilingShader false)
  (if (stale Custom|E_PerformShaderCompilation bIsLauncher)
    (Variables|Settings|SetbFirstShaderCompiled true)
    (Variables|/Game/HTML_Template/Save/Save_Shader.Save_Shader_C|SetbFirstShaderCompiled _save_shader true)
    (else
      (Utilities|Map|Add (Variables|Settings|GetCompiledLevelShader) (Variables|Settings|GetLevelAfterCompilation) true)
      (Utilities|Map|Add (Variables|/Game/HTML_Template/Save/Save_Shader.Save_Shader_C|GetCompiledLevelShader _save_shader) (Variables|Settings|GetLevelAfterCompilation) true)))
  (Save|SaveSettings (Variables|Save|GetSave_Shader) "NewEnumerator3")
  (Utilities|Array|Clear (Variables|Settings|GetCompilingShaderLevels))
  (Variables|Settings|SetCurrentLevelToCompile 0)
  (bind _loading_screen_widget (CallFunction|HandleLoadingScreen "NewEnumerator0"))
  (EventDispatchers|BindEventtoOnLoadingComplete _loading_screen_widget (delegate Custom|LoadingScreenProcessComplete))
  (Widget|RemovefromParent (Variables|Widget|GetShaderLoadingscreenWidget)))

(event Custom|LoadingScreenProcessComplete
  (Class|Html5Library|OpenLevel(byObjectReference) (Variables|Settings|GetLevelAfterCompilation)))

(event Custom|E_LevelToPreCompile
  (params (SelectedLevel :type World%20Soft%20Object%20Reference))
  ;[0 0 0] Level To Precompile From Game Instance
  (bind _loading_screen_widget (CallFunction|HandleLoadingScreen "NewEnumerator0"))
  (EventDispatchers|BindEventtoOnLoadingComplete _loading_screen_widget (delegate Custom|LoadingComplete)))

(event Custom|LoadingComplete
  ;[0 0 0] Level To Precompile From Game Instance
  (CallFunction|EPerformShaderCompilation (stale Custom|E_LevelToPreCompile SelectedLevel) false))

(event Custom|E_RedrawCompilerWidget
  (bind _shaderloadingscreenwidget (Variables|Widget|GetShaderLoadingscreenWidget))
  ;[0 0 0] Force Redraw Compiler Widget During Shader Compilation
  (Utilities|IsValid _shaderloadingscreenwidget
    (:Is%20Valid
      (UserInterface|Viewport|AddtoViewport _shaderloadingscreenwidget 0))))

(fn PlayMainMenuMusic
  (Utilities|IsValid (Variables|Audio|Music|GetMainMenuMusic)
    (:Is%20Valid
      (if (not (Variables|Audio|Music|GetbIsMainMenuMusicPlaying))
        (Variables|Audio|Music|SetbIsMainMenuMusicPlaying true)
        (bind _returnvalue (Audio|SpawnSound2D (Variables|Audio|Music|GetMainMenuMusic) 1.0 1.0 0.0 0 true false))
        (bind _output_get (Variables|Default|SetSound_MainMenuMusic _returnvalue))
        (Audio|Components|Audio|FadeIn _output_get 1.0 1.0 0.0 :!class /Script/Engine.AudioComponent)))))

(fn InitializeGameData
  (bind _gamedata (Variables|Default|GetGameData))
  (Variables|Audio|Music|SetMainMenuMusic (Variables|/Game/HTML_Template/Blueprint/Core/DataAsset/PDA_Game.PDA_Game_C|GetMainMenuMusic _gamedata))
  (Variables|Audio|Music|SetGameMusic (Variables|/Game/HTML_Template/Blueprint/Core/DataAsset/PDA_Game.PDA_Game_C|GetGameMusic _gamedata)))

(fn SetAudioSettings
  (params (bFadeAudio :type Boolean) (Fading%20Mode :type Enum_AudioFade%20Enum :default "NewEnumerator0") (FadingTime :type Float%20%28single-precision%29))
  (Variables|Audio|SetbIsAudioFade bFadeAudio)
  (LocalVariables|SetAudioFadingMode Fading%20Mode)
  (LocalVariables|SetAudioFadingTime FadingTime)
  (Variables|Save|SetSave_Audio (Save|GetAudioSavedSettings))
  (Utilities|FlowControl|Sequence
    (:then_0
      (if (not (Variables|Audio|GetbIsAudioFade))
        (LocalVariables|SetMixFadingTime 0.0)
        (LocalVariables|SetMusicVolume (Audio|AudioLogNormalization (Variables|/Game/HTML_Template/Save/Save_Audio.Save_Audio_C|GetMusic (Variables|Save|GetSave_Audio))) :!label _label)
        (LocalVariables|SetSoundEffectsVolume (Audio|AudioLogNormalization (Variables|/Game/HTML_Template/Save/Save_Audio.Save_Audio_C|GetSoundEffects (Variables|Save|GetSave_Audio))))
        (LocalVariables|SetMasterVolume (Audio|AudioLogNormalization (Variables|/Game/HTML_Template/Save/Save_Audio.Save_Audio_C|GetMasterAudio (Variables|Save|GetSave_Audio))))
        (else
          (LocalVariables|SetMixFadingTime FadingTime)
          (switch Utilities|FlowControl|Switch|SwitchonEnum_AudioFade Fading%20Mode
            (:NewEnumerator0
              (goto _label))
            (:NewEnumerator1
              (LocalVariables|SetMusicVolume 0.0)
              (LocalVariables|SetSoundEffectsVolume 0.0)
              (LocalVariables|SetMasterVolume 0.0))))))
    (:then_1
      ;[0 0 0] Music
      (Audio|SetSoundMixClassOverride "/Game/HTML_Template/Audio/SoundMix_Music.SoundMix_Music" "/Game/HTML_Template/Audio/SoundClass_Music.SoundClass_Music" (LocalVariables|GetMusicVolume) 1.0 (LocalVariables|GetMixFadingTime) false)
      (Audio|PushSoundMixModifier "/Game/HTML_Template/Audio/SoundMix_Music.SoundMix_Music")
      ;[0 0 0] Sound Effects
      (Audio|SetSoundMixClassOverride "/Game/HTML_Template/Audio/SoundMix_SoundEffect.SoundMix_SoundEffect" "/Game/HTML_Template/Audio/SoundClass_SoundEffect.SoundClass_SoundEffect" (LocalVariables|GetSoundEffectsVolume) 1.0 (LocalVariables|GetMixFadingTime) false)
      (Audio|PushSoundMixModifier "/Game/HTML_Template/Audio/SoundMix_SoundEffect.SoundMix_SoundEffect")
      ;[1 0.3624 0] Master
      (Audio|SetSoundMixClassOverride "/Game/HTML_Template/Audio/SoundMix_Master.SoundMix_Master" "/Game/HTML_Template/Audio/SoundClass_Master.SoundClass_Master" (LocalVariables|GetMasterVolume) 1.0 (LocalVariables|GetMixFadingTime) true)
      (Audio|PushSoundMixModifier "/Game/HTML_Template/Audio/SoundMix_Master.SoundMix_Master"))))

(fn SetVideoSettings
  (Variables|Save|SetSave_Video (Save|GetVideoSavedSettings))
  ;[0 0 0] Max FPS
  (switch Utilities|FlowControl|Switch|SwitchonEnum_Video_FramerateTarget (Variables|/Game/HTML_Template/Save/Save_Video.Save_Video_C|GetFramerate (Variables|Save|GetSave_Video))
    (:NewEnumerator0
      (Development|ExecuteConsoleCommand "t.maxfps 30" 0))
    (:NewEnumerator1
      (Development|ExecuteConsoleCommand "t.maxfps 60" 0)))
  ;[0 0 0] Anti-Aliasing
  (switch Utilities|FlowControl|Switch|SwitchonEnum_Video_AntiAliasing (Variables|/Game/HTML_Template/Save/Save_Video.Save_Video_C|GetAntiAliasing (Variables|Save|GetSave_Video))
    (:NewEnumerator0
      (Development|ExecuteConsoleCommand "r.AntiAliasingMethod 0" 0))
    (:NewEnumerator1
      (Development|ExecuteConsoleCommand "r.AntiAliasingMethod 3" 0)
      (Development|ExecuteConsoleCommand "r.MSAACount 2" 0))
    (:NewEnumerator4
      (Development|ExecuteConsoleCommand "r.AntiAliasingMethod 3" 0)
      (Development|ExecuteConsoleCommand "r.MSAACount 4" 0)))
  ;[0 0 0] Shadow Quality
  (switch Utilities|FlowControl|Switch|SwitchonEnum_Video_Shadow (Variables|/Game/HTML_Template/Save/Save_Video.Save_Video_C|GetShadow (Variables|Save|GetSave_Video))
    (:NewEnumerator0
      (Development|ExecuteConsoleCommand "sg.ShadowQuality 0" 0))
    (:NewEnumerator1
      (Development|ExecuteConsoleCommand "sg.ShadowQuality 1" 0))
    (:NewEnumerator4
      (Development|ExecuteConsoleCommand "sg.ShadowQuality 2" 0))
    (:NewEnumerator5
      (Development|ExecuteConsoleCommand "sg.ShadowQuality 3" 0)))
  ;[0 0 0] Texture Quality
  (switch Utilities|FlowControl|Switch|SwitchonEnum_Video_TextureQuality (Variables|/Game/HTML_Template/Save/Save_Video.Save_Video_C|GetTextureQuality (Variables|Save|GetSave_Video))
    (:NewEnumerator1
      (Development|ExecuteConsoleCommand "sg.TextureQuality 0" 0))
    (:NewEnumerator4
      (Development|ExecuteConsoleCommand "sg.TextureQuality 1" 0))
    (:NewEnumerator5
      (Development|ExecuteConsoleCommand "sg.TextureQuality 2" 0)))
  ;[0 0 0] Material Quality
  (switch Utilities|FlowControl|Switch|SwitchonEnum_Video_MaterialQuality (Variables|/Game/HTML_Template/Save/Save_Video.Save_Video_C|GetMaterialQuality (Variables|Save|GetSave_Video))
    (:NewEnumerator1
      (Development|ExecuteConsoleCommand "r.MaterialQualityLevel 0" 0))
    (:NewEnumerator4
      (Development|ExecuteConsoleCommand "r.MaterialQualityLevel 1" 0))
    (:NewEnumerator5
      (Development|ExecuteConsoleCommand "r.MaterialQualityLevel 2" 0)))
  ;[0 0 0] Bloom
  (switch Utilities|FlowControl|Switch|SwitchonEnum_Video_Bloom (Variables|/Game/HTML_Template/Save/Save_Video.Save_Video_C|GetBloom (Variables|Save|GetSave_Video))
    (:NewEnumerator0
      (Development|ExecuteConsoleCommand "r.BloomQuality 0" 0)
      (Development|ExecuteConsoleCommand "r.Bloom.ScreenPercentage 10" 0))
    (:NewEnumerator1
      (Development|ExecuteConsoleCommand "r.BloomQuality 2" 0)
      (Development|ExecuteConsoleCommand "r.Bloom.ScreenPercentage 25" 0))
    (:NewEnumerator4
      (Development|ExecuteConsoleCommand "r.BloomQuality 4" 0)
      (Development|ExecuteConsoleCommand "r.Bloom.ScreenPercentage 50" 0))
    (:NewEnumerator5
      (Development|ExecuteConsoleCommand "r.BloomQuality 5" 0)
      (Development|ExecuteConsoleCommand "r.Bloom.ScreenPercentage 100" 0)))
  ;[0 0 0] Screen Percent
  (switch Utilities|FlowControl|Switch|SwitchonEnum_Video_ScreenPercent (Variables|/Game/HTML_Template/Save/Save_Video.Save_Video_C|GetScreenPercent (Variables|Save|GetSave_Video))
    (:NewEnumerator4
      (Development|ExecuteConsoleCommand "r.ScreenPercentage 50" 0))
    (:NewEnumerator7
      (Development|ExecuteConsoleCommand "r.ScreenPercentage 60" 0))
    (:NewEnumerator8
      (Development|ExecuteConsoleCommand "r.ScreenPercentage 70" 0))
    (:NewEnumerator9
      (Development|ExecuteConsoleCommand "r.ScreenPercentage 80" 0))
    (:NewEnumerator10
      (Development|ExecuteConsoleCommand "r.ScreenPercentage 90" 0))
    (:NewEnumerator11
      (Development|ExecuteConsoleCommand "r.ScreenPercentage 100" 0))))

(fn GetSavedSettings
  (params (Save%20Type :type Enum_SaveType%20Enum :default "NewEnumerator0"))
  (LocalVariables|SetSlotName (Utilities|String|MakeLiteralString (Save|GetSaveName Save%20Type)))
  (bind _returnvalue (SaveGame|DoesSaveGameExist (LocalVariables|GetSlotName)))
  (if _returnvalue
    (bind _returnvalue_2 (SaveGame|LoadGamefromSlot (LocalVariables|GetSlotName)))
    (return true _returnvalue_2)
    (else
      (return false 0))))

(fn GetSaveName
  (params (Save%20Type :type Enum_SaveType%20Enum :default "NewEnumerator0"))
  (return (Utilities|String|Append (Class|Html5Library|GetProjectName) "_" "Save" "_" (Utilities|String|EnumtoString Save%20Type))))

(fn AudioLogNormalization
  (params (Volume :type Integer))
  (return (Math|Float|MapRangeClamped (Math|Conversions|ToFloat(Integer) Volume) 0.0 1e+02 0.0 1.0)))

(fn GetAudioSavedSettings
  (bind (_bloaded _gamesave) (Save|GetSavedSettings "NewEnumerator0"))
  (LocalVariables|SetSavedData _gamesave)
  (if _bloaded
    (Variables|Save|SetSave_Audio (.AsSave%20Audio (Utilities|Casting|CastToSave_Audio (LocalVariables|GetSavedData))))
    (else
      (bind _returnvalue (SaveGame|CreateSaveGameObject "/Game/HTML_Template/Save/Save_Audio.Save_Audio_C"))
      (Variables|Save|SetSave_Audio _returnvalue)))
  (return (Variables|Save|GetSave_Audio)))

(fn GetGameDataSavedSettings
  (bind (_bloaded _gamesave) (Save|GetSavedSettings "NewEnumerator4"))
  (LocalVariables|SetSavedData _gamesave)
  (if _bloaded
    (Variables|Save|SetSave_GameData (.AsSave%20Game%20Data (Utilities|Casting|CastToSave_GameData (LocalVariables|GetSavedData))))
    (else
      (bind _returnvalue (SaveGame|CreateSaveGameObject "/Game/HTML_Template/Save/Save_GameData.Save_GameData_C"))
      (Variables|Save|SetSave_GameData _returnvalue)))
  (return (Variables|Save|GetSave_GameData)))

(fn GetVideoSavedSettings
  (bind (_bloaded _gamesave) (Save|GetSavedSettings "NewEnumerator2"))
  (LocalVariables|SetSavedData _gamesave)
  (if _bloaded
    (Variables|Save|SetSave_Video (.AsSave%20Video (Utilities|Casting|CastToSave_Video (LocalVariables|GetSavedData))))
    (else
      (bind _returnvalue (SaveGame|CreateSaveGameObject "/Game/HTML_Template/Save/Save_Video.Save_Video_C"))
      (Variables|Save|SetSave_Video _returnvalue)))
  (return (Variables|Save|GetSave_Video)))

(fn GetShaderSavedSettings
  (bind (_bloaded _gamesave) (Save|GetSavedSettings "NewEnumerator3"))
  (LocalVariables|SetSavedData _gamesave)
  (if _bloaded
    (Variables|Save|SetSave_Shader (.AsSave%20Shader (Utilities|Casting|CastToSave_Shader (LocalVariables|GetSavedData))))
    (else
      (bind _returnvalue (SaveGame|CreateSaveGameObject "/Game/HTML_Template/Save/Save_Shader.Save_Shader_C"))
      (Variables|Save|SetSave_Shader _returnvalue)))
  (return (Variables|Save|GetSave_Shader)))

(fn GetPrivacySavedSettings
  (bind (_bloaded _gamesave) (Save|GetSavedSettings "NewEnumerator5"))
  (LocalVariables|SetSavedData _gamesave)
  (if _bloaded
    (Variables|Save|SetSave_Privacy (.AsSave%20Privacy (Utilities|Casting|CastToSave_Privacy (LocalVariables|GetSavedData))))
    (else
      (bind _returnvalue (SaveGame|CreateSaveGameObject "/Game/HTML_Template/Save/Save_Privacy.Save_Privacy_C"))
      (Variables|Save|SetSave_Privacy _returnvalue)))
  (return (Variables|Save|GetSave_Privacy)))

(fn SaveSettings
  (params (Save%20Game%20Object :type Save%20Game%20Object%20Reference) (Save%20Type :type Enum_SaveType%20Enum :default "NewEnumerator0"))
  (SaveGame|SaveGametoSlot Save%20Game%20Object (Save|GetSaveName Save%20Type)))

(fn ConfigureFirstSessionVideoSettings
  ;[0 0 0] First Video Settings - Max: Will Require Auto Benchmark
  (CallFunction|ConfigureVideoSettings "NewEnumerator1" "NewEnumerator4" "NewEnumerator5" "NewEnumerator5" "NewEnumerator5" "NewEnumerator5" "NewEnumerator11")
  (Save|SetVideoSettings))

(fn SaveVideoandApply
  (params (Save%20Video :type Save%20Video%20Object%20Reference) (bApply :type Boolean))
  (SaveGame|SaveGametoSlot Save%20Video (Save|GetSaveName "NewEnumerator2"))
  (if bApply
    (Save|SetVideoSettings)))

(fn FadeOutMainMenuMusic
  (bind _sound_mainmenumusic (Variables|Default|GetSound_MainMenuMusic))
  (if (Variables|Audio|Music|GetbIsMainMenuMusicPlaying)
    (Utilities|IsValid _sound_mainmenumusic
      (:Is%20Valid
        (Audio|Components|Audio|FadeOut _sound_mainmenumusic 1.0 0.0 :!class /Script/Engine.AudioComponent)
        (Utilities|Time|SetTimerbyFunctionName self "StopMainMenuMusic" 1.0)))))

(fn StopMainMenuMusic
  (Variables|Audio|Music|SetbIsMainMenuMusicPlaying false)
  (Utilities|IsValid (Variables|Default|GetSound_MainMenuMusic)
    (:Is%20Valid
      (Audio|Components|Audio|Stop (Variables|Default|GetSound_MainMenuMusic))
      (Variables|Default|SetSound_MainMenuMusic 0))))