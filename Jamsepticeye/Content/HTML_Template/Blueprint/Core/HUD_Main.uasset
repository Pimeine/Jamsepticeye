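; Main HUD Blueprint that shows and hides the pause menu and FPS counter widgets.
; On BeginPlay it restores FPS counter visibility from the GameInstance's SaveVideo object, and each toggle writes that flag back.
; Widgets are created on demand and cleared when hidden.
; The pause menu also switches input between Game-and-UI and Game-only, leaving the cursor visible in both cases.
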(event Custom|E_AddFramerateWidget
  (params (bIsVisible :type Boolean))
  ;[0 0 0] Add FPS Counter to HUD
  (if bIsVisible
    (Variables|Default|GetFpsCounterWidget
      (:then
        _)
      (:else
        (bind _returnvalue (UserInterface|CreateWidget "/Game/HTML_Template/Blueprint/Widget/AddOn/W_FpsCounter.W_FpsCounter_C"))
        (bind _output_get (Variables|Default|SetFpsCounterWidget _returnvalue))))
    (UserInterface|Viewport|AddtoViewport _output_get 100)
    (Variables|/Game/HTML_Template/Save/Save_Video.Save_Video_C|SetbShowFpsWidget (Variables|/Game/HTML_Template/Blueprint/Core/GI_HtmlGame.GI_HtmlGame_C|GetSave_Video (Variables|Default|GetGameInstance)) true)
    (else
      (bind _fpscounterwidget (Variables|Default|GetFpsCounterWidget)
        (:then
          (Widget|RemovefromParent _fpscounterwidget)
          (Variables|Default|SetFpsCounterWidget 0)
          (Variables|/Game/HTML_Template/Save/Save_Video.Save_Video_C|SetbShowFpsWidget (Variables|/Game/HTML_Template/Blueprint/Core/GI_HtmlGame.GI_HtmlGame_C|GetSave_Video (Variables|Default|GetGameInstance)) false))
        (:else)))))

(event EventBeginPlay
  (Variables|Default|SetGameInstance (CallFunction|GetMyGameInstance))
  (CallFunction|LoadSavedHUDSettings))

(event EventDisplayPauseMenu
  (params (bIsVisible :type Boolean))
  (bind _returnvalue (Game|GetPlayerController 0))
  (bind _returnvalue_2 (Game|GetPlayerController 0))
  ;[0 0 0] Create Pause Menu Widget
  (if bIsVisible
    (Variables|Default|GetPauseMenuWidget
      (:then
        _)
      (:else
        (bind _returnvalue_3 (UserInterface|CreateWidget "/Game/HTML_Template/Blueprint/Widget/Manager/Menu/WBP_PauseMenu.WBP_PauseMenu_C"))
        (bind _output_get (Variables|Default|SetPauseMenuWidget _returnvalue_3))))
    (UserInterface|Viewport|AddtoViewport _output_get 0)
    (Input|SetInputModeGameandUI _returnvalue_2 (Variables|Default|GetPauseMenuWidget) "DoNotLock" false)
    (Variables|/Script/Engine.PlayerController|SetbShowMouseCursor _returnvalue_2 true)
    (else
      (bind _pausemenuwidget (Variables|Default|GetPauseMenuWidget)
        (:then
          (Widget|RemovefromParent _pausemenuwidget)
          (Variables|Default|SetPauseMenuWidget 0)
          (Input|SetInputModeGameOnly _returnvalue)
          (Variables|/Script/Engine.PlayerController|SetbShowMouseCursor _returnvalue true))
        (:else)))))

(event EventDisplayFramerateCounter
  (params (bIsVisible :type Boolean))
  ;[0 0 0] Add FPS Counter to HUD
  (if bIsVisible
    (Variables|Default|GetFpsCounterWidget
      (:then
        _)
      (:else
        (bind _returnvalue (UserInterface|CreateWidget "/Game/HTML_Template/Blueprint/Widget/AddOn/W_FpsCounter.W_FpsCounter_C"))
        (bind _output_get (Variables|Default|SetFpsCounterWidget _returnvalue))))
    (UserInterface|Viewport|AddtoViewport _output_get 100)
    (Variables|/Game/HTML_Template/Save/Save_Video.Save_Video_C|SetbShowFpsWidget (Variables|/Game/HTML_Template/Blueprint/Core/GI_HtmlGame.GI_HtmlGame_C|GetSave_Video (Variables|Default|GetGameInstance)) true)
    (else
      (bind _fpscounterwidget (Variables|Default|GetFpsCounterWidget)
        (:then
          (Widget|RemovefromParent _fpscounterwidget)
          (Variables|Default|SetFpsCounterWidget 0)
          (Variables|/Game/HTML_Template/Save/Save_Video.Save_Video_C|SetbShowFpsWidget (Variables|/Game/HTML_Template/Blueprint/Core/GI_HtmlGame.GI_HtmlGame_C|GetSave_Video (Variables|Default|GetGameInstance)) false))
        (:else)))))

(fn ConstructionScript)

(fn LoadSavedHUDSettings
  (bind _gameinstance (Variables|Default|GetGameInstance))
  (bind _save_video (Variables|/Game/HTML_Template/Blueprint/Core/GI_HtmlGame.GI_HtmlGame_C|GetSave_Video _gameinstance))
  (Utilities|IsValid _save_video
    (:Is%20Valid
      (if (Variables|/Game/HTML_Template/Save/Save_Video.Save_Video_C|GetbShowFpsWidget _save_video)
        (CallFunction|EAddFramerateWidget true)
        (else
          (CallFunction|EAddFramerateWidget false))))))